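; Player resource component for the building system that links an inherited resource map to the player's UI and tracks the selected resource.
; InitializeManager stores the player, has the main widget generate per-resource widgets, then fills and highlights them.
; UpdateResourceDisplay extends the parent to refresh the matching widget's amount, and the main widget's current-resource display if selected.
; SelectNextResource changes the selected key index, moves the highlight, updates the main widget and fires OnResourceSwitch.
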(event `OnResourceSwitch`)

(event `InitializeManager`
  (params (Player :type "/Game/ThirdPerson/Blueprints/BP_ThirdPersonCharacter Object Reference"))
  (`/Engine/EditorBlueprintResources/StandardMacros.IsValid` Player
    (:`Is Valid`
      (set `self.PlayerCharacter` Player)
      (set `self.IsInitialized` true)
      (bind _createdwidgets (`/Game/BuildingSystem/Widgets/WBP_Main.GenerateResourceWidgets` (`/Game/ThirdPerson/Blueprints/BP_ThirdPersonCharacter.MainWidget` (`self.PlayerCharacter`)) self))
      (set `self.ResourceWidget` _createdwidgets)
      (`BlueprintMapLibrary.Map_Keys` (`self.Resources`))
      (for _array_element _
        (`self.UpdateResourceDisplay` _array_element))
      (`self.SelectCurrentResource`))))

(fn `CurrentlySelectedWidget`
  (returns (Widget :type "/Game/BuildingSystem/Widgets/WBP_Resource Object Reference"))
  (return (`.Widget` (`self.GetWidgetForResource` (`self.GetSelectedResource`)))))

(fn `GetSelectedIndex`
  (returns (Out :type Integer))
  (return (`self.SelectedResourceIndex`)))

(fn `GetSelectedResource`
  (returns (Out :type "/Game/BuildingSystem/Blueprints/Classes/BP_Master_Resource Class Reference"))
  (bind _keys (`BlueprintMapLibrary.Map_Keys` (`self.Resources`)))
  (return (`|GetArrayItem` _keys (`self.SelectedResourceIndex`))))

(fn `GetWidgetForResource`
  (params (Resource :type "/Game/BuildingSystem/Blueprints/Classes/BP_Master_Resource Class Reference"))
  (returns (IsSuccess :type Boolean) (Widget :type "/Game/BuildingSystem/Widgets/WBP_Resource Object Reference"))
  (locals (LocalFoundWidget :type "/Game/BuildingSystem/Widgets/WBP_Resource Object Reference"))
  (bind _localfoundwidget (`local.LocalFoundWidget`))
  (for _array_element (`self.ResourceWidget`)
    (if (== (`/Game/BuildingSystem/Widgets/WBP_Resource.Resource` _array_element) Resource)
      (set `local.LocalFoundWidget` _array_element)
      (break)))
  (`/Engine/EditorBlueprintResources/StandardMacros.IsValid` _localfoundwidget
    (:`Is Valid`
      (return true _localfoundwidget))
    (:`Is Not Valid`
      (return false null))))

(fn `SelectCurrentResource`
  (`/Game/BuildingSystem/Widgets/WBP_Resource.SelectResource` (`self.CurrentlySelectedWidget`) true false)
  (return))

(fn `SelectNextResource`
  (bind _selectedresourceindex (`self.SelectedResourceIndex`))
  (`/Game/BuildingSystem/Widgets/WBP_Resource.SelectResource` (`self.CurrentlySelectedWidget`) false false)
  (bind _keys (`BlueprintMapLibrary.Map_Keys` (`self.Resources`)))
  (set `self.SelectedResourceIndex` (`KismetMathLibrary.SelectInt` (+ _selectedresourceindex 1) 0 (< (`KismetArrayLibrary.Array_LastIndex` _keys) _selectedresourceindex)))
  (`self.SelectCurrentResource`)
  (`/Game/BuildingSystem/Widgets/WBP_Main.UpdateCurrentResource` (`/Game/ThirdPerson/Blueprints/BP_ThirdPersonCharacter.MainWidget` (`self.PlayerCharacter`)) self)
  (`self.OnResourceSwitch`))

(fn `UpdateResourceDisplay`
  (params (Resource :type "/Game/BuildingSystem/Blueprints/Classes/BP_Master_Resource Class Reference"))
  (bind (_issuccess _widget) (`self.GetWidgetForResource` Resource))
  (`parent.UpdateResourceDisplay` Resource)
  (if (`self.IsInitialized`)
    (if _issuccess
      (`TextBlock.SetText` (`/Game/BuildingSystem/Widgets/WBP_Resource.TXT_Amount` _widget) (`KismetTextLibrary.Conv_IntToText` (`self.GetResource` Resource) false false))
      (if (== Resource (`self.GetSelectedResource`))
        (`/Game/BuildingSystem/Widgets/WBP_Main.UpdateCurrentResource` (`/Game/ThirdPerson/Blueprints/BP_ThirdPersonCharacter.MainWidget` (`self.PlayerCharacter`)) self)))
    (else
      (return))))