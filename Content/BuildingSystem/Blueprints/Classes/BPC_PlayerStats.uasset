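; Player stats component that extends a parent stats class and links Health and Shield to their bars in the player's main widget.
; InitializeManager stores the player and runs stat setup, and OnStateSetUp then initializes the matching bar for each stat key with its StatValue.
; UpdateStat only calls the parent version, as the node that would refresh the bar with the current value is disconnected.
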(event `InitializeManager`
  (params (Player :type "/Game/ThirdPerson/Blueprints/BP_ThirdPersonCharacter Object Reference"))
  (set `self.PlayerRef` Player)
  (`self.SetUpState`))

(event `self.OnStateSetUp`
  (bind _keys (`BlueprintMapLibrary.Map_Keys` (`self.Stats`)))
  (for _array_element _keys
    (`/Game/BuildingSystem/Widgets/WBP_StatBar.InitializeBar` (`self.GetBarForStat` _array_element) (`.StatValue` (`self.GetStat` _array_element)))))

(fn `GetBarForStat`
  (params (Stat :type "/Game/BuildingSystem/Blueprints/Enums/E_Stats Enum" :default "NewEnumerator0"))
  (returns (Bar :type "/Game/BuildingSystem/Widgets/WBP_StatBar Object Reference"))
  (bind _mainwidget (`/Game/ThirdPerson/Blueprints/BP_ThirdPersonCharacter.MainWidget` (`self.PlayerRef`)))
  (return (select `/Game/BuildingSystem/Blueprints/Enums/E_Stats` Stat :`NewEnumerator1` (`/Game/BuildingSystem/Widgets/WBP_Main.WBP_ShieldBar` _mainwidget) :`NewEnumerator2` (`/Game/BuildingSystem/Widgets/WBP_Main.WBP_HealthBar` _mainwidget))))

(fn `UpdateStat`
  (params (Stat :type "/Game/BuildingSystem/Blueprints/Enums/E_Stats Enum" :default "NewEnumerator0"))
  (`parent.UpdateStat` Stat))