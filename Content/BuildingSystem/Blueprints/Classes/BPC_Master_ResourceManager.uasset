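; Master resource manager component for the building system, storing resource amounts in a map keyed by class.
; AddResource and RemoveResource validate input, write totals clamped to 0–999, then call UpdateResourceDisplay, an empty stub here.
; RemoveResource stores the requested amount minus the held value, the reverse of a normal subtraction.
; GetResource always returns 0, as its map lookup is disconnected.
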(fn `AddResource`
  (params (Resource :type "/Game/BuildingSystem/Blueprints/Classes/BP_Master_Resource Class Reference") (Amount :type Integer))
  (locals (LocalResource :type "/Game/BuildingSystem/Blueprints/Classes/BP_Master_Resource Class Reference") (LocalAmount :type Integer))
  (bind _resources (`self.Resources`))
  (bind _localresource (`local.LocalResource`))
  (bind (_value _returnvalue) (`BlueprintMapLibrary.Map_Find` (`self.Resources`) (`local.LocalResource`)))
  (set `local.LocalResource` Resource)
  (set `local.LocalAmount` Amount)
  (if (and (`KismetSystemLibrary.IsValidClass` Resource) (> Amount 0))
    (if _returnvalue
      (`BlueprintMapLibrary.Map_Add` _resources _localresource (`KismetMathLibrary.Clamp` (+ (`local.LocalAmount`) _value) 0 999))
      (else
        (`BlueprintMapLibrary.Map_Add` _resources _localresource (`KismetMathLibrary.Clamp` (`local.LocalAmount`) 0 999))))
    (`self.UpdateResourceDisplay` (`local.LocalResource`))
    (return)
    (else
      (return))))

(fn `GetResource`
  (params (Resource :type "/Game/BuildingSystem/Blueprints/Classes/BP_Master_Resource Class Reference"))
  (returns (Amount :type Integer))
  (return 0))

(fn `RemoveResource`
  (params (Resource :type "/Game/BuildingSystem/Blueprints/Classes/BP_Master_Resource Class Reference") (Amount :type Integer))
  (locals (LocalResource :type "/Game/BuildingSystem/Blueprints/Classes/BP_Master_Resource Class Reference") (LocalAmount :type Integer))
  (bind (_value _returnvalue) (`BlueprintMapLibrary.Map_Find` (`self.Resources`) (`local.LocalResource`)))
  (set `local.LocalResource` Resource)
  (set `local.LocalAmount` Amount)
  (if (and (`KismetSystemLibrary.IsValidClass` Resource) (> Amount 0))
    (if _returnvalue
      (`BlueprintMapLibrary.Map_Add` (`self.Resources`) (`local.LocalResource`) (`KismetMathLibrary.Clamp` (- (`local.LocalAmount`) _value) 0 999))
      (`self.UpdateResourceDisplay` (`local.LocalResource`))
      (return)
      (else
        (return)))
    (else
      (return))))

(fn `UpdateResourceDisplay`
  (params (Resource :type "/Game/BuildingSystem/Blueprints/Classes/BP_Master_Resource Class Reference")))