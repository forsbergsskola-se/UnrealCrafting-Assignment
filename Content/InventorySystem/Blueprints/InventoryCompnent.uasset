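; Inventory component that tracks item quantities in a map keyed by item.
; Adding sums onto the stored count, clamps the total to a fixed range and always reports success, even when the clamp discards some of the quantity.
; Querying returns the held amount and whether it covers the request.
; Removal relies on that query, subtracting only when enough is held and leaving emptied entries in the map.
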(fn `AddToInventory`
  (params (ItemToBeAdded :type "/Game/InventorySystem/Blueprints/Crafting/Item_Parent Class Reference") (Quantity :type Integer))
  (returns (Sucess :type Boolean))
  (`BlueprintMapLibrary.Map_Add` (`self.Inventory`) ItemToBeAdded (`KismetMathLibrary.Clamp` (+ Quantity (`BlueprintMapLibrary.Map_Find` (`self.Inventory`) ItemToBeAdded)) 0 99))
  (return true))

(fn `QueryInventory`
  (params (Item :type "/Game/InventorySystem/Blueprints/Crafting/Item_Parent Class Reference") (Quantity :type Integer))
  (returns (Amount :type Integer) (Success :type Boolean))
  (bind (_value _returnvalue) (`BlueprintMapLibrary.Map_Find` (`self.Inventory`) Item))
  (if (and (>= _value Quantity) _returnvalue)
    (return _value true)
    (else
      (return _value false))))

(fn `RemoveFromInventory`
  (params (ItemToBeRemoved :type "/Game/InventorySystem/Blueprints/Crafting/Item_Parent Class Reference") (Quantity :type Integer))
  (returns (Success :type Boolean))
  (bind (_amount _success) (`self.QueryInventory` ItemToBeRemoved Quantity))
  (if _success
    (`BlueprintMapLibrary.Map_Add` (`self.Inventory`) (`local.ItemToBeRemoved`) (- _amount (`local.Quantity`)))
    (return true)
    (else
      (return false))))