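; Item_Parent is a pickup actor for the inventory and crafting system, apparently meant as a base class for items.
; On Interactwith, it adds one of its own class to the interacting character's inventory component.
; It then casts player 0 to BP_ThirdPersonCharacter, refreshes the inventory in that character's crafting menu and destroys itself.
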(event `/Game/InventorySystem/Blueprints/IF_Interact.InteractWith`
  (params (PlayerCharacter :type "/Game/ThirdPerson/Blueprints/BP_ThirdPersonCharacter Object Reference"))
  (`/Game/InventorySystem/Blueprints/InventoryCompnent.AddToInventory` (`/Game/ThirdPerson/Blueprints/BP_ThirdPersonCharacter.InventoryCompnent` PlayerCharacter) (`GameplayStatics.GetObjectClass` self) 1)
  (bind _asbp_third_person_character (cast `/Game/ThirdPerson/Blueprints/BP_ThirdPersonCharacter` (`GameplayStatics.GetPlayerCharacter` 0)))
  (`/Engine/EditorBlueprintResources/StandardMacros.IsValid` _asbp_third_person_character
    (:`Is Valid`
      (`/Game/InventorySystem/Blueprints/UI/CraftingMenu.Refresh Inventory` (`/Game/BuildingSystem/Widgets/WBP_Main.CraftingMenu` (`/Game/ThirdPerson/Blueprints/BP_ThirdPersonCharacter.MainWidget` _asbp_third_person_character)))
      (`self.K2_DestroyActor`))))

(fn `UserConstructionScript`)